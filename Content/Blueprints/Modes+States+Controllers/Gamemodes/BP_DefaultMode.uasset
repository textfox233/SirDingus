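; Default game mode with GameStart and GameOver events, where GameStart is an empty stub.
; GameOver ignores its PlayerVictory flag and calls AddWidgetToServer on player 0's BP_PlayerCharacter.
; The mode's own AddWidgetToServer relays to AddWidgetToClient, which shows a new WBP_EndGame regardless of its inputs, but GameOver never calls this pair.
; Win/lose text, start screen and in-progress reset logic sit in disconnected nodes that never run.
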(event `self.GameStart`)

(event `self.GameOver`
  (params (bPlayerVictory :type Boolean))
  (bind _asbp_player_character (cast `/Game/Blueprints/Characters/BP_PlayerCharacter` (`GameplayStatics.GetPlayerCharacter` 0)))
  (`/Game/Blueprints/Characters/BP_PlayerCharacter.Add Widget To Server` _asbp_player_character))

(event `Add Widget To Server`
  (params (Widget :type "UserWidget Object Reference") (WidgetClass :type "UserWidget Class Reference"))
  (`self.Add Widget To Client` Widget WidgetClass))

(event `Add Widget To Client`
  (params (Widget :type "UserWidget Object Reference") (WidgetClass :type "UserWidget Class Reference"))
  (bind _returnvalue (`|CreateWidget` "/Game/Blueprints/UI/WBP_EndGame.WBP_EndGame_C"))
  (`UserWidget.AddToViewport` _returnvalue 0))

(fn `UserConstructionScript`)