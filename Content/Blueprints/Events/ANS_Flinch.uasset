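; Anim notify state that sets a pawn's action state to Interrupted for the duration of a flinch animation window, then to Unoccupied when it ends.
; Both notify events use a shared helper that requires the mesh owner to be a locally controlled pawn whose controller implements ActionStateInterface.
; State changes go to the controller as interface messages, and each failed check prints a debug message.
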(fn `Check For Interface`
  (params (`Mesh Owner` :type "ActorComponent Object Reference"))
  (returns (`Object is Valid` :type Boolean) (`Interface Object` :type "Controller Object Reference"))
  ;[1 1 1] Check Pawn
  (bind _aspawn (cast `Pawn` (`ActorComponent.GetOwner` `Mesh Owner`))
    (:`then`
      ;[1 1 1] Check Local Control
      (if (`Pawn.IsLocallyControlled` _aspawn)
        (bind _returnvalue (`Pawn.GetController` _aspawn))
        ;[1 1 1] Check Interface
        (if (`KismetSystemLibrary.DoesImplementInterface` _returnvalue "/Script/SirDingus.ActionStateInterface")
          (return true _returnvalue)
          (else
            (`KismetSystemLibrary.PrintString` null "ERROR in ANS_Flinch::NotifyBegin - Target's owning controller does not implement the Action State interface" (`self.Interface`))
            (return false null)))
        (else
          (`KismetSystemLibrary.PrintString` null "ANS_Flinch::NotifyBegin - Target is not locally controlled" (`self.Local Control`) false)
          (return false null))))
    (:`CastFailed`
      (`KismetSystemLibrary.PrintString` null "ERROR in ANS_Flinch::NotifyBegin - Target is not a pawn (has no controller)" (`self.Pawn`) false)
      (return false null))))

(fn `Received_NotifyBegin`
  (params (MeshComp :type "SkeletalMeshComponent Object Reference") (Animation :type "AnimSequenceBase Object Reference") (TotalDuration :type "Float (single-precision)") (EventReference :type "AnimNotifyEventReference Structure (by ref)"))
  (returns (ReturnValue :type Boolean))
  (bind (_object_is_valid _interface_object) (`self.Check For Interface` MeshComp))
  (if _object_is_valid
    (message `ActionStateInterface.UpdateActionState` _interface_object "EAS_Interrupted")
    (return false)))

(fn `Received_NotifyEnd`
  (params (MeshComp :type "SkeletalMeshComponent Object Reference") (Animation :type "AnimSequenceBase Object Reference") (EventReference :type "AnimNotifyEventReference Structure (by ref)"))
  (returns (ReturnValue :type Boolean))
  (bind (_object_is_valid _interface_object) (`self.Check For Interface` MeshComp))
  (if _object_is_valid
    (message `ActionStateInterface.UpdateActionState` _interface_object "EAS_Unoccupied")
    (return false)))