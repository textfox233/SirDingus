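; Dungeon character Blueprint for great sword melee attacks, with EventGraph logic marked as deprecated in favor of C++.
; TriggerMelee starts a looping timer that traces the weapon arc with debug drawing and processes valid hits until StopTriggerMelee clears it.
; AttackEvent calls AttackBasic, which plays the vertical slash through PlayAnimMontageServer.
; Older server-to-client montage events with DoOnce gating remain, alongside disconnected damage and death reaction nodes.
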(event `TriggerMelee`
  ;[1 1 1] Deprecated, now implented in C++
  ;;[1 1 1] Start Line Tracing
  (bind _returnvalue (`KismetSystemLibrary.K2_SetTimerDelegate` (delegate `MeleeLineTrace`) 0.01 true))
  (set `self.TriggerMeleeEvent` _returnvalue))

(event `StopTriggerMelee`
  ;[1 1 1] Deprecated, now implented in C++
  ;;[1 1 1] Stop Line Tracing
  (`KismetSystemLibrary.K2_ClearAndInvalidateTimerHandle` (`self.TriggerMeleeEvent`)))

(event `MeleeLineTrace`
  ;[1 1 1] Deprecated, now implented in C++
  ;;[1 1 1] Melee Line Trace
  (bind _returnvalue (`self.DrawWeaponArc` true))
  (if (`KismetSystemLibrary.IsValid` _returnvalue)
    (`self.ProcessMeleeHit` _returnvalue)))

(event `Play Montage On Client`
  (params (InputPin :type "AnimMontage Object Reference"))
  ;[1 1 1] Deprecated, now implented in C++
  ;;[1 1 1] Play AnimMontages
  (`/Engine/EditorBlueprintResources/StandardMacros.DoOnce` false :!label _label
    (:`Completed`
      (bind _returnvalue (`self.PlayAnimMontage` InputPin))
      (`KismetSystemLibrary.Delay` _returnvalue)
      (goto _label :!via `Reset`))))

(event `self.AttackEvent`
  ;[1 1 1] Deprecated, now implented in C++
  ;;[1 1 1] Trigger Attack Animation
  (`self.AttackBasic`))

(event `Play Montage On Server`
  (params (AnimMontage :type "AnimMontage Object Reference"))
  ;[1 1 1] Deprecated, now implented in C++
  ;;[1 1 1] Play AnimMontages
  (`self.Play Montage On Client` AnimMontage))

(fn `AttackBasic`
  (`self.PlayAnimMontageServer` "/Game/Blueprints/Characters/Animation/Great_Sword_Slash_Vertical_Montage.Great_Sword_Slash_Vertical_Montage"))

(fn `UserConstructionScript`)