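; MeleeTraceEvent is an animation notify state that marks the melee trace window within an attack animation.
; On begin, it casts the mesh owner to BP_DungeonCharacter and calls TriggerMelee; on end, it calls StopTriggerMelee on the same cast.
; The tracing itself is left to the character, and a failed cast only prints an error.
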(fn `Received_NotifyBegin`
  (params (MeshComp :type "SkeletalMeshComponent Object Reference") (Animation :type "AnimSequenceBase Object Reference") (TotalDuration :type "Float (single-precision)") (EventReference :type "AnimNotifyEventReference Structure (by ref)"))
  (returns (ReturnValue :type Boolean))
  ;[1 1 1] Trigger Melee Trace Event
  (bind _asbp_dungeon_character (cast `/Game/Blueprints/Characters/BP_DungeonCharacter` (`ActorComponent.GetOwner` MeshComp))
    (:`then`
      (`/Game/Blueprints/Characters/BP_PlayerCharacter.TriggerMelee` _asbp_dungeon_character)
      (return false))
    (:`CastFailed`
      (`KismetSystemLibrary.PrintString` null "ERROR in MeleeEvent::NotifyBegin - Target is not BP_DungeonCharacter"))))

(fn `Received_NotifyEnd`
  (params (MeshComp :type "SkeletalMeshComponent Object Reference") (Animation :type "AnimSequenceBase Object Reference") (EventReference :type "AnimNotifyEventReference Structure (by ref)"))
  (returns (ReturnValue :type Boolean))
  ;[1 1 1] Stop Trigger Melee Event
  (bind _asbp_dungeon_character (cast `/Game/Blueprints/Characters/BP_DungeonCharacter` (`ActorComponent.GetOwner` MeshComp))
    (:`then`
      (`/Game/Blueprints/Characters/BP_PlayerCharacter.StopTriggerMelee` _asbp_dungeon_character)
      (return false))
    (:`CastFailed`
      (`KismetSystemLibrary.PrintString` null "ERROR in MeleeEvent::NotifyEnd - Target is not BP_DungeonCharacter"))))